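; Dev dialogue-system sprite character that combines cursor-aimed movement logic with a proximity dialogue trigger.
; Tick sets velocity from movement input at half walk speed, flips the sprite toward the cursor and rotates the shooting components gathered by the construction script.
; When BP_TestActor overlaps the Box, it shows Text and creates a DialogueUI widget, reversing both on exit.
; DialogueEvent and ResetDialogue only drive a DoOnce with nothing after it.
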(event `self.ReceiveTick`
  (params (DeltaSeconds :type "Float (single-precision)"))
  (bind _sprite (`self.Sprite`))
  (bind _charactermovement (`self.CharacterMovement`))
  (bind (_returnvalue_roll _returnvalue_pitch _returnvalue_yaw) (`KismetMathLibrary.BreakRotator` (`KismetMathLibrary.FindLookAtRotation` (`self.K2_GetActorLocation`) (`.Location` (`GameplayStatics.BreakHitResult` (`PlayerController.GetHitResultUnderCursorByChannel` (`GameplayStatics.GetPlayerController` 0) "TraceTypeQuery1" false))))))
  (set `MovementComponent.Velocity` (* (`KismetMathLibrary.Normal` (`KismetMathLibrary.MakeVector` (`self.GetInputAxisValue`) (* (`self.GetInputAxisValue`) -1.0))) (`CharacterMovementComponent.MaxWalkSpeed` _charactermovement) 0.5) _charactermovement)
  (`|ExecutionSequence`
    (:`then_0`
      (if (>= (`KismetMathLibrary.Abs` _returnvalue_yaw) 90.0)
        (`SceneComponent.K2_SetRelativeRotation` _sprite (`KismetMathLibrary.MakeRotator` -90.0 180.0) false false)
        (for _array_element (`self.ShootingComponents`)
          (`SceneComponent.K2_SetRelativeRotation` _array_element (`KismetMathLibrary.MakeRotator` 0.0 (+ _returnvalue_yaw 180.0)) false false))
        (else
          (`SceneComponent.K2_SetRelativeRotation` _sprite (`KismetMathLibrary.MakeRotator` -90.0) false false)
          (for _array_element_2 (`self.ShootingComponents`)
            (`SceneComponent.K2_SetRelativeRotation` _array_element_2 (`KismetMathLibrary.MakeRotator` 0.0 (* _returnvalue_yaw -1.0)) false false)))))))

(event `self.Box.OnComponentBeginOverlap`
  (params (OverlappedComponent :type "PrimitiveComponent Object Reference") (OtherActor :type "Actor Object Reference") (OtherComp :type "PrimitiveComponent Object Reference") (OtherBodyIndex :type Integer) (bFromSweep :type Boolean) (SweepResult :type "HitResult Structure (by ref)"))
  ;[1 1 1] Sistema de Diálogo(Luís)
  (cast `/Game/Bin/Blueprints/Character/BP_TestActor` OtherActor)
  (`SceneComponent.SetHiddenInGame` (`self.Text`) false false)
  (bind _returnvalue (`|CreateWidget` "/Game/Dev/Luís/DialogueSystem/DialogueUI.DialogueUI_C" (`GameplayStatics.GetPlayerController` 0)))
  (bind _output_get (set `self.DialogueUI` _returnvalue))
  (`UserWidget.AddToViewport` _output_get 0))

(event `self.Box.OnComponentEndOverlap`
  (params (OverlappedComponent :type "PrimitiveComponent Object Reference") (OtherActor :type "Actor Object Reference") (OtherComp :type "PrimitiveComponent Object Reference") (OtherBodyIndex :type Integer))
  (bind _dialogueui (`self.DialogueUI`))
  ;[1 1 1] Sistema de Diálogo(Luís)
  (cast `/Game/Bin/Blueprints/Character/BP_TestActor` OtherActor)
  (`SceneComponent.SetHiddenInGame` (`self.Text`) true false)
  (`/Engine/EditorBlueprintResources/StandardMacros.IsValid` _dialogueui
    (:`Is Valid`
      (`Widget.RemoveFromParent` _dialogueui))))

(event `/Game/Dev/Luís/DialogueSystem/DialogueInterface.Dialogue Event`
  ;[1 1 1] Sistema de Diálogo(Luís)
  (`/Engine/EditorBlueprintResources/StandardMacros.DoOnce` false :!label _label))

(event `ResetDialogue`
  ;[1 1 1] Sistema de Diálogo(Luís)
  (goto _label :!via `Reset`))

(fn `UserConstructionScript`
  (`parent.UserConstructionScript`)
  (for _array_element (`SceneComponent.GetChildrenComponents` (`self.Sprite`) true)
    (if (== (`GameplayStatics.GetObjectClass` _array_element) "/Game/Bin/Blueprints/Character/BP_Shooting_Component.BP_Shooting_Component_C")
      (bind _asbp_shooting_component (cast `/Game/Bin/Blueprints/Character/BP_Shooting_Component` _array_element))
      (`KismetArrayLibrary.Array_AddUnique` (`self.ShootingComponents`) _asbp_shooting_component))))