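; Test actor for a player-controlled group of four child-actor heroes that moves by pivoting around its left or right hero.
; The Move Left/Right axis re-parents the other heroes and two cylinders to Hero 2 (right) or Hero 4 (left), then yaws that pivot.
; Move actions toggle run and flip sprites, re-centering the actor on the pivot upon release.
; Temporary action inputs make Heroes 2 and 4 shoot projectiles.
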(event `self.ReceiveBeginPlay`
  (bind _asbp_test_hero_base (cast `/Game/Dev/Gibran/BP_TestHeroBase` (`ChildActorComponent.ChildActor` (`self.cHero1`))))
  (set `self.Hero1` _asbp_test_hero_base)
  (bind _asbp_test_hero_base_2 (cast `/Game/Dev/Gibran/BP_TestHeroBase` (`ChildActorComponent.ChildActor` (`self.cHero2`))))
  (set `self.Hero2` _asbp_test_hero_base_2)
  (bind _asbp_test_hero_base_3 (cast `/Game/Dev/Gibran/BP_TestHeroBase` (`ChildActorComponent.ChildActor` (`self.cHero3`))))
  (set `self.Hero3` _asbp_test_hero_base_3)
  (bind _asbp_test_hero_base_4 (cast `/Game/Dev/Gibran/BP_TestHeroBase` (`ChildActorComponent.ChildActor` (`self.cHero4`))))
  (set `self.Hero4` _asbp_test_hero_base_4))

(event `self.ReceiveTick`
  (params (DeltaSeconds :type "Float (single-precision)")))

(event `InputAxis|Move Left/Right`
  (params (AxisValue :type "Float (single-precision)"))
  (bind _cylinder (`self.Cylinder`))
  (bind _chero2 (`self.cHero2`))
  (bind _cylinder1 (`self.Cylinder1`))
  (bind _chero1 (`self.cHero1`))
  (bind _chero4 (`self.cHero4`))
  (bind _chero3 (`self.cHero3`))
  (bind _returnvalue (* (* AxisValue (`GameplayStatics.GetWorldDeltaSeconds`)) 150.0))
  ;[0 0 0] Dettaches the components from each other first
  (`SceneComponent.K2_DetachFromComponent` (`self.cHero1`) "KeepWorld" "KeepWorld" "KeepRelative" true)
  (`SceneComponent.K2_DetachFromComponent` (`self.cHero2`) "KeepWorld" "KeepWorld" "KeepRelative" true)
  (`SceneComponent.K2_DetachFromComponent` (`self.cHero3`) "KeepWorld" "KeepWorld" "KeepRelative" true)
  (`SceneComponent.K2_DetachFromComponent` (`self.cHero4`) "KeepWorld" "KeepWorld" "KeepRelative" true)
  (`SceneComponent.K2_DetachFromComponent` (`self.Cylinder`) "KeepWorld" "KeepWorld" "KeepRelative" true)
  (`SceneComponent.K2_DetachFromComponent` (`self.Cylinder1`) "KeepWorld" "KeepWorld" "KeepRelative" true)
  ;[0 0 0] Attaches 3 of the heroes to a 4th one and rotates it
  (if (>= AxisValue 0.0)
    ;;[0 0 0] Attaches the heroes and rotates them around the right one
    (`SceneComponent.K2_AttachToComponent` _chero1 _chero2 "None" "KeepWorld" "KeepWorld" "KeepRelative" true)
    (`SceneComponent.K2_AttachToComponent` _chero3 _chero2 "None" "KeepWorld" "KeepWorld" "KeepRelative" true)
    (`SceneComponent.K2_AttachToComponent` _chero4 _chero2 "None" "KeepWorld" "KeepWorld" "KeepRelative" true)
    (`SceneComponent.K2_AttachToComponent` _cylinder _chero2 "None" "KeepWorld" "KeepWorld" "KeepRelative" true)
    (`SceneComponent.K2_AttachToComponent` _cylinder1 _chero2 "None" "KeepWorld" "KeepWorld" "KeepRelative" true)
    (`SceneComponent.K2_AddLocalRotation` _chero2 (`KismetMathLibrary.MakeRotator` 0.0 0.0 _returnvalue) false false)
    (else
      ;;[0 0 0] Attaches the heroes and rotates them around the left one
      (`SceneComponent.K2_AttachToComponent` _chero1 _chero4 "None" "KeepWorld" "KeepWorld" "KeepRelative" true)
      (`SceneComponent.K2_AttachToComponent` _chero2 _chero4 "None" "KeepWorld" "KeepWorld" "KeepRelative" true)
      (`SceneComponent.K2_AttachToComponent` _chero3 _chero4 "None" "KeepWorld" "KeepWorld" "KeepRelative" true)
      (`SceneComponent.K2_AttachToComponent` _cylinder _chero4 "None" "KeepWorld" "KeepWorld" "KeepRelative" true)
      (`SceneComponent.K2_AttachToComponent` _cylinder1 _chero4 "None" "KeepWorld" "KeepWorld" "KeepRelative" true)
      (`SceneComponent.K2_AddLocalRotation` _chero4 (`KismetMathLibrary.MakeRotator` 0.0 0.0 _returnvalue) false false))))

(event `InputAction|aMoveLeft`
  (params (Key :type "Key Structure"))
  (bind _hero2 (`self.Hero2`))
  (bind _chero4 (`self.cHero4`))
  (bind _hero3 (`self.Hero3`))
  (bind _hero1 (`self.Hero1`))
  (:`Pressed`
    ;[0 0 0] *temporary* Moves the sprites of the characters
    (`/Game/Dev/Gibran/BP_TestHeroBase.SpriteRun` _hero1)
    (`/Game/Dev/Gibran/BP_TestHeroBase.SpriteFlip` _hero1 -2.0)
    (`/Game/Dev/Gibran/BP_TestHeroBase.SpriteRun` _hero2)
    (`/Game/Dev/Gibran/BP_TestHeroBase.SpriteFlip` _hero2 -2.0)
    (`/Game/Dev/Gibran/BP_TestHeroBase.SpriteRun` _hero3)
    (`/Game/Dev/Gibran/BP_TestHeroBase.SpriteFlip` _hero3 -2.0)
    (`/Game/Dev/Gibran/BP_TestHeroBase.SpriteFlip` (`self.Hero4`) -2.0))
  (:`Released`
    ;[0 0 0] Resets the position of the group actor to the unmoved character
    (bind _output_get (set `self.TmpWorldLocation` (`SceneComponent.K2_GetComponentLocation` _chero4)))
    (`self.K2_SetActorLocation` _output_get)
    (`SceneComponent.K2_SetWorldLocation` _chero4 _output_get false false)
    (`/Game/Dev/Gibran/BP_TestHeroBase.SpriteStop` (`self.Hero1`) :!label _label)
    (`/Game/Dev/Gibran/BP_TestHeroBase.SpriteStop` (`self.Hero2`))
    (`/Game/Dev/Gibran/BP_TestHeroBase.SpriteStop` (`self.Hero3`))
    (`/Game/Dev/Gibran/BP_TestHeroBase.SpriteStop` (`self.Hero4`))))

(event `InputAction|aMoveRight`
  (params (Key :type "Key Structure"))
  (bind _chero2 (`self.cHero2`))
  (bind _hero4 (`self.Hero4`))
  (bind _hero3 (`self.Hero3`))
  (bind _hero1 (`self.Hero1`))
  (:`Pressed`
    ;[0 0 0] *temporary* Moves the sprites of the characters
    (`/Game/Dev/Gibran/BP_TestHeroBase.SpriteRun` _hero1)
    (`/Game/Dev/Gibran/BP_TestHeroBase.SpriteFlip` _hero1 2.0)
    (`/Game/Dev/Gibran/BP_TestHeroBase.SpriteRun` _hero3)
    (`/Game/Dev/Gibran/BP_TestHeroBase.SpriteFlip` _hero3 2.0)
    (`/Game/Dev/Gibran/BP_TestHeroBase.SpriteRun` _hero4)
    (`/Game/Dev/Gibran/BP_TestHeroBase.SpriteFlip` _hero4 2.0)
    (`/Game/Dev/Gibran/BP_TestHeroBase.SpriteFlip` (`self.Hero2`) 2.0))
  (:`Released`
    ;[0 0 0] Resets the position of the group actor to the unmoved character
    (bind _output_get (set `self.TmpWorldLocation` (`SceneComponent.K2_GetComponentLocation` _chero2)))
    (`self.K2_SetActorLocation` _output_get)
    (`SceneComponent.K2_SetWorldLocation` _chero2 _output_get false false)
    (goto _label)))

(event `InputAction|Action 4`
  (params (Key :type "Key Structure"))
  ;[0 0 0] *temporary* Imput for the characters actions
  (:`Pressed`
    (`/Game/Bin/Blueprints/Character/BP_Shooting_Component.Shoot Once Projectile Class` (`/Game/Dev/Gibran/BP_TestHeroBase.BP_Shooting_Component` (`self.Hero4`)) null)))

(event `InputAction|Action 2`
  (params (Key :type "Key Structure"))
  ;[0 0 0] *temporary* Imput for the characters actions
  (:`Pressed`
    (`/Game/Bin/Blueprints/Character/BP_Shooting_Component.Shoot Once Projectile Class` (`/Game/Dev/Gibran/BP_TestHeroBase.BP_Shooting_Component` (`self.Hero2`)) null)))

(fn `UserConstructionScript`)