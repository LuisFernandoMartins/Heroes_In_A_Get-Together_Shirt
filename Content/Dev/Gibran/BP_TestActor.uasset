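; Test actor that swings a formation of four BP_TestHero child actors left or right around one of its members.
; Every axis update detaches heroes and cylinders, reattaches them to CHero2 (zero or positive input) or CHero4 (negative), then yaws that pivot by the input.
; Left/right presses flip all sprites and start run animations on all but the pivot hero; releases stop all four.
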(event `self.ReceiveBeginPlay`
  (bind _asbp_test_hero (cast `/Game/Dev/Gibran/BP_TestHero` (`ChildActorComponent.ChildActor` (`self.cHero1`))))
  (set `self.Hero1` _asbp_test_hero)
  (bind _asbp_test_hero_2 (cast `/Game/Dev/Gibran/BP_TestHero` (`ChildActorComponent.ChildActor` (`self.cHero2`))))
  (set `self.Hero2` _asbp_test_hero_2)
  (bind _asbp_test_hero_3 (cast `/Game/Dev/Gibran/BP_TestHero` (`ChildActorComponent.ChildActor` (`self.cHero3`))))
  (set `self.Hero3` _asbp_test_hero_3)
  (bind _asbp_test_hero_4 (cast `/Game/Dev/Gibran/BP_TestHero` (`ChildActorComponent.ChildActor` (`self.cHero4`))))
  (set `self.Hero4` _asbp_test_hero_4))

(event `self.ReceiveTick`
  (params (DeltaSeconds :type "Float (single-precision)")))

(event `InputAxis|Move Left/Right`
  (params (AxisValue :type "Float (single-precision)"))
  (bind _returnvalue (* AxisValue 2.0))
  (bind _cylinder (`self.Cylinder`))
  (bind _chero2 (`self.cHero2`))
  (bind _cylinder1 (`self.Cylinder1`))
  (bind _chero1 (`self.cHero1`))
  (bind _chero4 (`self.cHero4`))
  (bind _chero3 (`self.cHero3`))
  (`SceneComponent.K2_DetachFromComponent` (`self.cHero1`) "KeepWorld" "KeepWorld" "KeepRelative" true)
  (`SceneComponent.K2_DetachFromComponent` (`self.cHero2`) "KeepWorld" "KeepWorld" "KeepRelative" true)
  (`SceneComponent.K2_DetachFromComponent` (`self.cHero3`) "KeepWorld" "KeepWorld" "KeepRelative" true)
  (`SceneComponent.K2_DetachFromComponent` (`self.cHero4`) "KeepWorld" "KeepWorld" "KeepRelative" true)
  (`SceneComponent.K2_DetachFromComponent` (`self.Cylinder`) "KeepWorld" "KeepWorld" "KeepRelative" true)
  (`SceneComponent.K2_DetachFromComponent` (`self.Cylinder1`) "KeepWorld" "KeepWorld" "KeepRelative" true)
  (if (>= AxisValue 0.0)
    (`SceneComponent.K2_AttachToComponent` _chero1 _chero2 "None" "KeepWorld" "KeepWorld" "KeepRelative" true)
    (`SceneComponent.K2_AttachToComponent` _chero4 _chero2 "None" "KeepWorld" "KeepWorld" "KeepRelative" true)
    (`SceneComponent.K2_AttachToComponent` _chero3 _chero2 "None" "KeepWorld" "KeepWorld" "KeepRelative" true)
    (`SceneComponent.K2_AttachToComponent` _cylinder _chero2 "None" "KeepWorld" "KeepWorld" "KeepRelative" true)
    (`SceneComponent.K2_AttachToComponent` _cylinder1 _chero2 "None" "KeepWorld" "KeepWorld" "KeepRelative" true)
    (`SceneComponent.K2_AddLocalRotation` _chero2 (`KismetMathLibrary.MakeRotator` 0.0 0.0 _returnvalue) false false)
    (else
      (`SceneComponent.K2_AttachToComponent` _chero1 _chero4 "None" "KeepWorld" "KeepWorld" "KeepRelative" true)
      (`SceneComponent.K2_AttachToComponent` _chero2 _chero4 "None" "KeepWorld" "KeepWorld" "KeepRelative" true)
      (`SceneComponent.K2_AttachToComponent` _chero3 _chero4 "None" "KeepWorld" "KeepWorld" "KeepRelative" true)
      (`SceneComponent.K2_AttachToComponent` _cylinder _chero4 "None" "KeepWorld" "KeepWorld" "KeepRelative" true)
      (`SceneComponent.K2_AttachToComponent` _cylinder1 _chero4 "None" "KeepWorld" "KeepWorld" "KeepRelative" true)
      (`SceneComponent.K2_AddLocalRotation` _chero4 (`KismetMathLibrary.MakeRotator` 0.0 0.0 _returnvalue) false false))))

(event `InputAction|aMoveLeft`
  (params (Key :type "Key Structure"))
  (bind _hero1 (`self.Hero1`))
  (bind _hero2 (`self.Hero2`))
  (bind _hero4 (`self.Hero4`))
  (bind _hero3 (`self.Hero3`))
  (:`Pressed`
    (`/Game/Dev/Gibran/BP_TestHero.SpriteRun` _hero1)
    (`/Game/Dev/Gibran/BP_TestHero.SpriteFlip` _hero1 -2.0)
    (`/Game/Dev/Gibran/BP_TestHero.SpriteRun` _hero2)
    (`/Game/Dev/Gibran/BP_TestHero.SpriteFlip` _hero2 -2.0)
    (`/Game/Dev/Gibran/BP_TestHero.SpriteRun` _hero3)
    (`/Game/Dev/Gibran/BP_TestHero.SpriteFlip` _hero3 -2.0)
    (`/Game/Dev/Gibran/BP_TestHero.SpriteFlip` _hero4 -2.0))
  (:`Released`
    (`/Game/Dev/Gibran/BP_TestHero.SpriteStop` _hero1 :!label _label)
    (`/Game/Dev/Gibran/BP_TestHero.SpriteStop` _hero2)
    (`/Game/Dev/Gibran/BP_TestHero.SpriteStop` _hero3)
    (`/Game/Dev/Gibran/BP_TestHero.SpriteStop` _hero4)))

(event `InputAction|aMoveRight`
  (params (Key :type "Key Structure"))
  (bind _hero1 (`self.Hero1`))
  (bind _hero4 (`self.Hero4`))
  (bind _hero3 (`self.Hero3`))
  (:`Pressed`
    (`/Game/Dev/Gibran/BP_TestHero.SpriteRun` _hero1)
    (`/Game/Dev/Gibran/BP_TestHero.SpriteFlip` _hero1 2.0)
    (`/Game/Dev/Gibran/BP_TestHero.SpriteRun` _hero3)
    (`/Game/Dev/Gibran/BP_TestHero.SpriteFlip` _hero3 2.0)
    (`/Game/Dev/Gibran/BP_TestHero.SpriteRun` _hero4)
    (`/Game/Dev/Gibran/BP_TestHero.SpriteFlip` _hero4 2.0)
    (`/Game/Dev/Gibran/BP_TestHero.SpriteFlip` (`self.Hero2`) 2.0))
  (:`Released`
    (goto _label)))

(fn `UserConstructionScript`)