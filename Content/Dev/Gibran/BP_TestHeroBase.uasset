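; Test hero base Blueprint, apparently used as a child actor, that shows a 2D flipbook character with a number label and icon and can fire projectiles.
; Tick holds the flipbook at a fixed world rotation, reads the parent actor's velocity to switch idle and run animations, and mirrors the sprite through negative X scale.
; InitShooting starts a looping timer at the BulletsPerSecond rate that fires through BPShootingComponent.
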(event `self.ReceiveTick`
  (params (DeltaSeconds :type "Float (single-precision)"))
  (bind _returnvalue (`self.GetVelocity` (`self.GetParentActor`)))
  (`SceneComponent.K2_SetWorldRotation` (`self.Flipbook`) (struct :`Roll` -90.0) false false)
  (if (== (`KismetMathLibrary.VSize` _returnvalue) 0.0)
    (`self.SpriteStop`)
    (else
      (if (> (.x _returnvalue) 0.0)
        (`self.SpriteFlip` 2.0)
        (else
          (`self.SpriteFlip` -2.0)))
      (`self.SpriteRun`))))

(event `self.ReceiveBeginPlay`
  (`TextRenderComponent.K2_SetText` (`self.NumberText`) (`KismetTextLibrary.Conv_IntToText` (`self.Number`)))
  (`BillboardComponent.SetSprite` (`self.Icon`) (`self.IconTxt`))
  (`PaperFlipbookComponent.SetFlipbook` (`self.Flipbook`) (`self.IdleFlipbook`)))

(event `SpriteRun`
  (`PaperFlipbookComponent.SetFlipbook` (`self.Flipbook`) (`self.RunFlipbook`)))

(event `Init Shooting`
  (`KismetSystemLibrary.K2_SetTimerDelegate` (delegate `Shoot`) (/ 1.0 (`self.BulletsPerSecond`)) true))

(event `SpriteStop`
  (`PaperFlipbookComponent.SetFlipbook` (`self.Flipbook`) (`self.IdleFlipbook`)))

(event `Shoot`
  (`/Game/Bin/Blueprints/Character/BP_Shooting_Component.Shoot Once Projectile Class` (`self.BP_Shooting_Component`) null))

(event `SpriteFlip`
  (params (Scale :type "Float (double-precision)"))
  (`SceneComponent.SetRelativeScale3D` (`self.Flipbook`) (`KismetMathLibrary.MakeVector` Scale 2.0 2.0)))

(fn `UserConstructionScript`)