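; Test spawner that populates a box volume with a set number of BP_TestDrone actors.
; On BeginPlay it spawns the drones at random XY points at the box's center height, registering itself as each one's spawner.
; DroneDestroyed removes the drone from the tracked array and spawns a replacement.
; A looping timer counts all test drones in the world and calls DestroyDrone on any excess.
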(event `DroneDestroyed`
  (params (Drone :type "/Game/Dev/Gibran/BP_TestDrone Object Reference"))
  (bind (_origin _boxextent) (`KismetSystemLibrary.GetComponentBounds` (`self.Box`)))
  (bind (_returnvalue_x _returnvalue_y) (`KismetMathLibrary.BreakVector` (`KismetMathLibrary.RandomPointInBoundingBox` _origin _boxextent)))
  (`/Engine/EditorBlueprintResources/StandardMacros.IsValid` Drone
    (:`Is Valid`
      (`KismetArrayLibrary.Array_RemoveItem` (`self.Drones`) Drone))
    (:`Is Not Valid`
      _))
  (bind _returnvalue (`|SpawnActorFromClass` "/Game/Dev/Gibran/BP_TestDrone.BP_TestDrone_C" (`KismetMathLibrary.MakeTransform` (`KismetMathLibrary.MakeVector` _returnvalue_x _returnvalue_y (.z _origin))) "AdjustIfPossibleButAlwaysSpawn" "OverrideRootScale" null null :!label _label))
  (set `/Game/Dev/Gibran/BP_TestDrone.Spawner` self _returnvalue)
  (`KismetArrayLibrary.Array_Add` (`self.Drones`) _returnvalue))

(event `self.ReceiveBeginPlay`
  (`KismetSystemLibrary.K2_SetTimerDelegate` (delegate `CheckDroneAmmount`) 2.0 true)
  (for _ (range 1 (+ (`self.DroneNumber`) 1))
    (goto _label)))

(event `CheckDroneAmmount`
  (bind _dronenumber (`self.DroneNumber`))
  (bind _outactors (`GameplayStatics.GetAllActorsOfClass` "/Game/Dev/Gibran/BP_TestDrone.BP_TestDrone_C"))
  (bind _returnvalue (`KismetArrayLibrary.Array_Length` _outactors))
  (if (> _returnvalue _dronenumber)
    (for _index (range (- _returnvalue _dronenumber))
      (`/Game/Dev/Gibran/BP_TestDrone.DestroyDrone` (`|GetArrayItem` _outactors _index)))))

(fn `UserConstructionScript`)