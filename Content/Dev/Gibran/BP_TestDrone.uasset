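; Test drone actor that wanders at a fixed height, fires periodically and dies from any damage.
; Looping timers with randomized intervals drive both behaviors, with a timeline sized to the wander interval lerping it toward nearby navmesh-sampled positions without sweep.
; Each shot gives the ShootingComponent a random relative yaw before firing once.
; On destruction it notifies its Spawner, then removes itself after a short delay.
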(event `DestroyDrone`
  (`/Game/Dev/Gibran/BP_TestDroneSpawner.DroneDestroyed` (`self.Spawner`) self :!label _label)
  (`KismetSystemLibrary.Delay` 0.2)
  (`self.K2_DestroyActor`))

(event `self.ReceiveAnyDamage`
  (params (Damage :type "Float (single-precision)") (DamageType :type "DamageType Object Reference") (InstigatedBy :type "Controller Object Reference") (DamageCauser :type "Actor Object Reference"))
  (goto _label))

(event `self.ReceiveBeginPlay`
  (bind _returnvalue (`KismetMathLibrary.RandomFloatInRange` 0.5 2.5))
  (bind _output_get (set `self.WanderingTime` _returnvalue))
  (`KismetSystemLibrary.K2_SetTimerDelegate` (delegate `Wander`) _output_get true)
  (`TimelineComponent.SetTimelineLength` (`self.Timeline_0`) _output_get)
  (`KismetSystemLibrary.K2_SetTimerDelegate` (delegate `Shoot`) _returnvalue true))

(event `Shoot`
  (bind _shooting_component (`self.Shooting_Component`))
  (`SceneComponent.K2_SetRelativeRotation` _shooting_component (`KismetMathLibrary.MakeRotator` -90.0 0.0 (`KismetMathLibrary.RandomFloatInRange` 0.0 360.0)) false false)
  (`/Game/Bin/Blueprints/Character/BP_Shooting_Component.ShootOnce` _shooting_component))

(event `Wander`
  (bind _returnvalue (`self.K2_GetActorLocation`))
  (bind _randomlocation (`NavigationSystemV1.K2_GetRandomLocationInNavigableRadius` _returnvalue 200.0 null null))
  (bind _output_get (set `self.PreviousPosition` _returnvalue))
  (bind _output_get_2 (set `self.NewPosition` (`KismetMathLibrary.MakeVector` (.x _randomlocation) (.y _randomlocation) (`.Z` (`KismetMathLibrary.BreakVector3f` _returnvalue)))))
  (bind (_direction _alfa) (`Timeline|Timeline_0` :!via `PlayFromStart`)
    (:`Update`
      (`self.K2_SetActorLocation` (`KismetMathLibrary.VLerp` _output_get _output_get_2 _alfa)))))

(fn `UserConstructionScript`)