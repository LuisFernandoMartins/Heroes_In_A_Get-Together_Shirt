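; BP_TestHero is a test hero Blueprint that shows a 2D flipbook character with a number label and an icon sprite.
; BeginPlay fills the text and icon from its variables and starts the idle flipbook.
; SpriteRun, SpriteStop and SpriteFlip events swap run and idle animations or set the X scale for facing.
; Tick forces a fixed world rotation on the flipbook, keeping its orientation independent of the actor's.
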(event `self.ReceiveTick`
  (params (DeltaSeconds :type "Float (single-precision)"))
  (`SceneComponent.K2_SetWorldRotation` (`self.Flipbook`) (struct :`Yaw` 90.0 :`Roll` -90.0) false false))

(event `self.ReceiveBeginPlay`
  (`TextRenderComponent.K2_SetText` (`self.NumberText`) (`KismetTextLibrary.Conv_IntToText` (`self.Number`)))
  (`BillboardComponent.SetSprite` (`self.Icon`) (`self.IconTxt`))
  (`PaperFlipbookComponent.SetFlipbook` (`self.Flipbook`) (`self.IdleFlipbook`)))

(event `SpriteRun`
  (`PaperFlipbookComponent.SetFlipbook` (`self.Flipbook`) (`self.RunFlipbook`)))

(event `SpriteStop`
  (`PaperFlipbookComponent.SetFlipbook` (`self.Flipbook`) (`self.IdleFlipbook`)))

(event `SpriteFlip`
  (params (Scale :type "Float (double-precision)"))
  (`SceneComponent.SetRelativeScale3D` (`self.Flipbook`) (`KismetMathLibrary.MakeVector` Scale 2.0 2.0)))

(fn `UserConstructionScript`)