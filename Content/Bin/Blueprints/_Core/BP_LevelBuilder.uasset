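; BP_LevelBuilder is a one-shot actor that populates a level from tilemap tile user data at BeginPlay.
; It scans every layer and cell, using the text before any comma as the tile type.
; Grass and Water tiles spawn overlays tagged with their type, while Emitter tiles spawn emitters whose particle sprite comes from the text after the comma.
; Spawns sit at tile centers in world space, and the builder destroys itself afterwards.
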(event `self.ReceiveBeginPlay`
  (bind _rendercomponent (`PaperTileMapActor.RenderComponent` (`self.Tilemap`)))
  (bind (_mapwidth _mapheight _numlayers) (`PaperTileMapComponent.GetMapSize` _rendercomponent))
  (for _index (range 1 (+ _numlayers 1))
    (for _index_2 (range 1 (+ _mapwidth 1))
      (for _index_3 (range 1 (+ _mapheight 1))
        (bind _returnvalue (`TileMapBlueprintLibrary.GetTileUserData` (`PaperTileMapComponent.GetTile` _rendercomponent _index_2 _index_3 _index)))
        (bind _returnvalue_2 (`KismetStringLibrary.Conv_NameToString` _returnvalue))
        (bind (_lefts _rights _returnvalue_3) (`KismetStringLibrary.Split` _returnvalue_2 ","))
        (switch `string` (`KismetMathLibrary.SelectString` _lefts _returnvalue_2 _returnvalue_3)
          (:`Grass`
            (bind _returnvalue_4 (`PaperTileMapComponent.GetTileCenterPosition` _rendercomponent _index_2 _index_3 _index true))
            (bind _returnvalue_5 (`|SpawnActorFromClass` "/Game/Bin/Blueprints/Misc/Overlay.Overlay_C" (`KismetMathLibrary.MakeTransform` _returnvalue_4) "Undefined" "OverrideRootScale" null null :!label _label))
            (set `/Game/Bin/Blueprints/Misc/Overlay.OverlayType` (`KismetStringLibrary.Conv_NameToString` _returnvalue) _returnvalue_5))
          (:`Water`
            (goto _label))
          (:`Emitter`
            (switch `string` _rights
              (:`Flower`
                _)
              (:`Leaf`
                _))
            (bind _returnvalue_6 (`|SpawnActorFromClass` "/Game/Bin/Blueprints/Misc/Emitter.Emitter_C" (`KismetMathLibrary.MakeTransform` _returnvalue_4) "Undefined" "OverrideRootScale" null null))
            (set `/Game/Bin/Blueprints/Misc/Emitter.ParticleSprite` _rights _returnvalue_6))))))
  (`self.K2_DestroyActor`))

(fn `UserConstructionScript`)