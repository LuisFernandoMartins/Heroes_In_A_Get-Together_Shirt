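; BP_Controller is a player controller that relays movement to the controlled pawn and marks the cursor's aim point.
; RotateMessage draws a debug sphere at the Visibility hit under the cursor, then sends MoveMessage to the pawn with normalized LR/UD axis input.
; A look-at control rotation toward the cursor is disconnected, and the Tick, axis and shooting handlers are empty.
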(event `InputAxis|LR`
  (params (AxisValue :type "Float (single-precision)")))

(event `InputAxis|UD`
  (params (AxisValue :type "Float (single-precision)")))

(event `self.ReceiveTick`
  (params (DeltaSeconds :type "Float (single-precision)")))

(event `InputAction|Shoot`
  (params (Key :type "Key Structure")))

(fn `UserConstructionScript`)