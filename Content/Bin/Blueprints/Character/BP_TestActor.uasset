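; BP_TestActor is a player-controlled sprite character that moves, shoots toward the mouse cursor and triggers dialogue.
; Tick sets velocity directly from movement axes, flips the sprite by cursor yaw and rotates the shooting components gathered from the sprite's children at construction.
; Holding left mouse fires every component, gated by a looping fire-rate timer.
; Pressing E messages the first overlapping actor implementing DialogueInterface.
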(event `self.ReceiveTick`
  (params (DeltaSeconds :type "Float (single-precision)"))
  (bind _sprite (`self.Sprite`))
  (bind _charactermovement (`self.CharacterMovement`))
  (bind (_returnvalue_roll _returnvalue_pitch _returnvalue_yaw) (`KismetMathLibrary.BreakRotator` (`KismetMathLibrary.FindLookAtRotation` (`self.K2_GetActorLocation`) (`.Location` (`GameplayStatics.BreakHitResult` (`PlayerController.GetHitResultUnderCursorByChannel` (`GameplayStatics.GetPlayerController` 0) "TraceTypeQuery1" false))))))
  (set `MovementComponent.Velocity` (* (`KismetMathLibrary.Normal` (`KismetMathLibrary.MakeVector` (`self.GetInputAxisValue`) (* (`self.GetInputAxisValue`) -1.0))) (`CharacterMovementComponent.MaxWalkSpeed` _charactermovement) 0.5) _charactermovement)
  (`|ExecutionSequence`
    (:`then_0`
      (if (>= (`KismetMathLibrary.Abs` _returnvalue_yaw) 90.0)
        (`SceneComponent.K2_SetRelativeRotation` _sprite (`KismetMathLibrary.MakeRotator` -90.0 180.0) false false)
        (for _array_element (`self.ShootingComponents`)
          (`SceneComponent.K2_SetRelativeRotation` _array_element (`KismetMathLibrary.MakeRotator` 0.0 (+ _returnvalue_yaw 180.0)) false false))
        (else
          (`SceneComponent.K2_SetRelativeRotation` _sprite (`KismetMathLibrary.MakeRotator` -90.0) false false)
          (for _array_element_2 (`self.ShootingComponents`)
            (`SceneComponent.K2_SetRelativeRotation` _array_element_2 (`KismetMathLibrary.MakeRotator` 0.0 (* _returnvalue_yaw -1.0)) false false)))))
    (:`then_1`
      (if (and (`PlayerController.IsInputKeyDown` (`GameplayStatics.GetPlayerController` 0) "LeftMouseButton") (`self.canshoot`))
        (for _array_element_3 (`self.ShootingComponents`)
          (`/Game/Bin/Blueprints/Character/BP_Shooting_Component.Shoot Once Projectile Class` _array_element_3 null))
        (set `self.canshoot` false)))))

(event `Key|LeftMouseButton`
  (params (Key :type "Key Structure")))

(event `self.ReceiveBeginPlay`
  (`self.EnableInput` (`GameplayStatics.GetPlayerController` 0))
  (`KismetSystemLibrary.K2_SetTimerDelegate` (delegate `reset time`) (/ 1.0 (`self.Firerate`)) true))

(event `reset time`
  (set `self.canshoot` true))

(event `Key|E`
  (params (Key :type "Key Structure"))
  ;[1 1 1] Luís
  (:`Pressed`
    (for _array_element (`self.GetOverlappingActors` null)
      (if (`KismetSystemLibrary.DoesImplementInterface` _array_element "/Game/Dev/Luís/DialogueSystem/DialogueInterface.DialogueInterface_C")
        (message `/Game/Dev/Luís/DialogueSystem/DialogueInterface.Dialogue Event` _array_element)
        (break)))))

(fn `UserConstructionScript`
  (`parent.UserConstructionScript`)
  (for _array_element (`SceneComponent.GetChildrenComponents` (`self.Sprite`) true)
    (if (== (`GameplayStatics.GetObjectClass` _array_element) "/Game/Bin/Blueprints/Character/BP_Shooting_Component.BP_Shooting_Component_C")
      (bind _asbp_shooting_component (cast `/Game/Bin/Blueprints/Character/BP_Shooting_Component` _array_element))
      (`KismetArrayLibrary.Array_AddUnique` (`self.ShootingComponents`) _asbp_shooting_component))))