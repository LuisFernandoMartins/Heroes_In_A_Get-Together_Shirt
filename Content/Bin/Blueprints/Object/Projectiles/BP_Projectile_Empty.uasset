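; Blank projectile Blueprint whose identity, look, motion and damage are supplied at runtime through a parameter struct.
; SetVariables copies name, speed, damage and damage type, and applies the sprite and color.
; It also swaps the trajectory curve into the Movement timeline's MovementCurve track and sets play rate to the inverse of lifespan, stretching the curve over the projectile's life.
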(event `Set Variables`
  (params (Params :type "/Game/Bin/Blueprints/Object/Projectiles/Struct_Projectile Structure"))
  (bind (_name _sprite _color _trajectory _speed _lifespan _damage _damagetype) (break `/Game/Bin/Blueprints/Object/Projectiles/Struct_Projectile` Params))
  (bind _movement (`self.Movement`))
  (set `self.Name` _name)
  (`self.Set New Sprite` _sprite _color)
  (`TimelineComponent.SetVectorCurve` _movement _trajectory "MovementCurve")
  (`TimelineComponent.SetPlayRate` _movement (/ 1.0 _lifespan))
  (set `self.Speed` _speed)
  (set `self.Damage` _damage)
  (set `self.DamageType` _damagetype))

(fn `UserConstructionScript`
  (`parent.UserConstructionScript`))