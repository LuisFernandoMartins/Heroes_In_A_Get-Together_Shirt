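; BP_Projectile_Straight_Spread is a projectile that bursts into a radial ring of smaller fragments when it dies.
; On death it asks the GameMode to spawn one BP_Projectile_Straight per Spreads count, spaced evenly in yaw with random jitter.
; Each fragment spawns at half scale with the fragment sprite and Parent passed as shooter, then the parent death logic runs.
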(event `self.OnDeath`
  (for _index (range 1 (+ (`self.Spreads`) 1))
    (bind _newbullet (message `/Game/Bin/Blueprints/_Core/BPI_GMBullet.RequestSpawnProjectile` (`GameplayStatics.GetGameMode`) "/Game/Bin/Blueprints/Object/Projectiles/BP_Projectile_Straight.BP_Projectile_Straight_C" (`KismetMathLibrary.MakeTransform` (.location (`self.GetTransform`)) (`KismetMathLibrary.ComposeRotators` (.rotation (`self.GetTransform`)) (`KismetMathLibrary.MakeRotator` 0.0 0.0 (+ (* _index (/ 360.0 (`KismetMathLibrary.Conv_IntToDouble` (`self.Spreads`)))) (`KismetMathLibrary.RandomFloatInRange` -15.0 15.0)))) (* (.scale (`self.GetTransform`)) 0.5)) (`self.Parent`)))
    (`self.Set New Sprite` _newbullet (`self.FragmentSprite`)))
  (`parent.OnDeath`))

(fn `UserConstructionScript`
  (`parent.UserConstructionScript`))