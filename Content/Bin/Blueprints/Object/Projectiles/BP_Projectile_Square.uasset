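; Projectile variant that, as its name suggests, travels a square path by turning 90 degrees at the end of each leg.
; BeginPlay quarters the inherited Lifespan before running the parent logic, so each leg gets a quarter of it.
; A non-looping MultiGate intercepts DestroyBullet, rotating and reactivating the projectile three times, then passing the fourth call to the parent's destroy logic.
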(event `self.ReceiveBeginPlay`
  (set `self.Lifespan` (/ (`self.Lifespan`) 4.0))
  (`parent.ReceiveBeginPlay`))

(event `self.DestroyBullet`
  (`|MultiGate` false
    (:`Out 0`
      (`self.K2_AddActorWorldRotation` (struct :`Yaw` 90.0) :!label _label)
      (`self.Activate`))
    (:`Out 1`
      (goto _label))
    (:`Out 2`
      (goto _label))
    (:`Out 3`
      (`parent.DestroyBullet`))))

(fn `UserConstructionScript`
  (`parent.UserConstructionScript`))