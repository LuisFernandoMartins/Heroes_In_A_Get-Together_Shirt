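; Sprite-based projectile that follows a vector curve trajectory and damages the first overlapping actor not tagged with its team.
; A Lifespan-long timeline scales the curve by Speed and Lifespan, mapping X to facing-direction travel, Y to up-vector offset and Z to yaw swing.
; Activate and Deactivate control movement and a hit gate.
; Impact or timeline end notifies the GameMode instead of destroying the actor directly.
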(event `Set New Sprite`
  (params (NewSprite :type "PaperSprite Object Reference"))
  (`PaperSpriteComponent.SetSprite` (`self.SpriteComponent`) NewSprite))

(event `self.ReceiveBeginPlay`
  (bind _movement (`self.Movement`))
  (`TimelineComponent.SetVectorCurve` _movement (`self.Trajectory`) "MovementCurve")
  (`TimelineComponent.SetPlayRate` _movement (/ 1.0 (`self.Lifespan`)))
  (`self.Set New Sprite` (`self.Sprite`)))

(event `Update`
  (params (NewLocation :type "Vector Structure"))
  (`self.K2_SetActorLocation` NewLocation))

(event `Activate`
  (set `self.InitPos` (`self.K2_GetActorLocation`))
  (`|ExecutionSequence`
    (:`then_0`
      (bind (_direction _movementcurve) (`Timeline|Movement` :!via `PlayFromStart` :!label _label)
        (:`Update`
          (`self.Update` (`self.Calculate Location` _movementcurve)))
        (:`Finished`
          (`self.OnDeath`))))
    (:`then_1`
      (goto _label_2 :!via `Open`))))

(event `Deactivate`
  (`|ExecutionSequence`
    (:`then_0`
      (goto _label :!via `Stop`))
    (:`then_1`
      (goto _label_2 :!via `Close`))))

(event `DestroyBullet`
  (message `/Game/Bin/Blueprints/_Core/BPI_GMBullet.ProjectileDied` (`GameplayStatics.GetGameMode`) self))

(event `self.SpriteComponent.OnComponentBeginOverlap`
  (params (OverlappedComponent :type "PrimitiveComponent Object Reference") (OtherActor :type "Actor Object Reference") (OtherComp :type "PrimitiveComponent Object Reference") (OtherBodyIndex :type Integer) (bFromSweep :type Boolean) (SweepResult :type "HitResult Structure (by ref)"))
  (`/Engine/EditorBlueprintResources/StandardMacros.IsValid` OtherActor
    (:`Is Valid`
      (if (not (`KismetArrayLibrary.Array_Contains` (`Actor.Tags` OtherActor) (`self.Team`)))
        (`/Engine/EditorBlueprintResources/StandardMacros.Gate` true :!label _label_2
          (:`Exit`
            (`GameplayStatics.ApplyDamage` OtherActor (`self.Damage`) (`self.GetInstigatorController` (`self.Parent`)) self (`self.DamageType`))
            (`self.OnDeath`)))))))

(event `OnDeath`
  (`self.DestroyBullet`))

(fn `Calculate Location`
  (params (`Vector Track` :type "Vector Structure"))
  (returns (ReturnValue :type "Vector Structure"))
  (bind (_returnvalue_roll _returnvalue_pitch _returnvalue_yaw) (`KismetMathLibrary.BreakRotator` (`self.K2_GetActorRotation`)))
  (return (+ (`self.InitPos`) (`KismetMathLibrary.RotateAngleAxis` (+ (`KismetMathLibrary.GreaterGreater_VectorRotator` (`KismetMathLibrary.MakeVector` (.x (* (`self.Lifespan`) (`self.Speed`) `Vector Track`))) (`KismetMathLibrary.MakeRotator` 0.0 0.0 _returnvalue_yaw)) (* (`self.GetActorUpVector`) (.y (* (`self.Lifespan`) (`self.Speed`) `Vector Track`)) 0.5)) (.z (* (`self.Lifespan`) (`self.Speed`) `Vector Track`)) (0.0 0.0 1.0)))))

(fn `UserConstructionScript`)