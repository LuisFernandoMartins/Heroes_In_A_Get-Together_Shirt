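; Team-aware projectile that follows a curve-driven path, damages actors it overlaps and can be activated and deactivated.
; A Movement timeline's vector curve, scaled by Lifetime and Speed, sets forward offset, height and rotation around Z from the launch point.
; While active, a gate passes sprite overlaps with actors lacking the Team tag into damage.
; Hits and timeline completion both notify the GameMode that the bullet died.
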(event `Activate`
  (`|ExecutionSequence`
    (:`then_0`
      (set `self.InitialLocation` (`self.K2_GetActorLocation`))
      (bind (_direction _movementcurve) (`Timeline|Movement` :!via `PlayFromStart` :!label _label)
        (:`Update`
          (`self.K2_SetActorLocation` (`self.Calculate Location` _movementcurve) true))
        (:`Finished`
          (`self.Die`))))
    (:`then_1`
      (goto _label_3 :!via `Open`))))

(event `Deactivate`
  (`|ExecutionSequence`
    (:`then_0`
      (goto _label :!via `Stop`))
    (:`then_1`
      (goto _label_3 :!via `Close`))))

(event `Die`
  (message `/Game/Bin/Blueprints/_Core/BPI_GamemodeBulletInteraction.BulletDied` (`GameplayStatics.GetGameMode`) self :!label _label_2))

(event `self.ReceiveActorBeginOverlap`
  (params (OtherActor :type "Actor Object Reference")))

(event `self.Sprite.OnComponentBeginOverlap`
  (params (OverlappedComponent :type "PrimitiveComponent Object Reference") (OtherActor :type "Actor Object Reference") (OtherComp :type "PrimitiveComponent Object Reference") (OtherBodyIndex :type Integer) (bFromSweep :type Boolean) (SweepResult :type "HitResult Structure (by ref)"))
  (`KismetSystemLibrary.PrintString` (`KismetSystemLibrary.GetDisplayName` OtherActor))
  (`/Engine/EditorBlueprintResources/StandardMacros.IsValid` OtherActor
    (:`Is Valid`
      (if (not (`KismetArrayLibrary.Array_Contains` (`Actor.Tags` OtherActor) (`self.Team`)))
        (`/Engine/EditorBlueprintResources/StandardMacros.Gate` true :!label _label_3
          (:`Exit`
            (`GameplayStatics.ApplyDamage` OtherActor (`self.Damage`) (`self.GetInstigatorController` (`self.Parent`)) self (`self.DamageType`))
            (goto _label_2)))))))

(fn `Calculate Location`
  (params (`Vector Track` :type "Vector Structure"))
  (returns (ReturnValue :type "Vector Structure"))
  (bind (_returnvalue_roll _returnvalue_pitch _returnvalue_yaw) (`KismetMathLibrary.BreakRotator` (`self.K2_GetActorRotation`)))
  (return (+ (`self.InitialLocation`) (`KismetMathLibrary.RotateAngleAxis` (+ (`KismetMathLibrary.GreaterGreater_VectorRotator` (`KismetMathLibrary.MakeVector` (.x (* (`self.Lifetime`) (`self.Speed`) `Vector Track`))) (`KismetMathLibrary.MakeRotator` 0.0 0.0 _returnvalue_yaw)) (* (`self.GetActorUpVector`) (.y (* (`self.Lifetime`) (`self.Speed`) `Vector Track`)))) (.z (* (`self.Lifetime`) (`self.Speed`) `Vector Track`)) (0.0 0.0 1.0)))))

(fn `UserConstructionScript`)